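; BP_StartLine is the lap-counting start/finish line trigger for the player's BP_Kart, which it caches on BeginPlay.
; Each overlap saves the lap time and calls EndLap and StartRace on the kart, then starts another lap or, if RaceComplete is set, ends the race.
; Both paths update the lap count after a short delay; completion later shows WB_RaceComplete.
; An unconnected per-lap time recording chain never runs.
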(event OnComponentBeginOverlap(StartLine)
  (params (OverlappedComponent :type Primitive%20Component%20Object%20Reference) (OtherActor :type Actor%20Object%20Reference) (OtherComp :type Primitive%20Component%20Object%20Reference) (OtherBodyIndex :type Integer) (bFromSweep :type Boolean) (SweepResult :type Hit%20Result%20Structure%20%28by%20ref%29))
  (bind _as_bp_kart_0 (Variables|Default|GetAs%20BP%20Kart_0))
  (bind _as_bp_kart_0_2 (Variables|Default|GetAs%20BP%20Kart_0))
  (bind _as_bp_kart_0_3 (Variables|Default|GetAs%20BP%20Kart_0))
  (Variables|Default|SetSavedLapTime (Variables|/Game/Vehicles/BP_Kart.BP_Kart_C|GetLapTimeAsText (Variables|Default|GetAs%20BP%20Kart_0)))
  (Default|EndLap _as_bp_kart_0)
  (Default|StartRace _as_bp_kart_0)
  (if (Variables|/Game/Vehicles/BP_Kart.BP_Kart_C|GetRaceComplete? _as_bp_kart_0_3)
    (Utilities|FlowControl|Delay 0.4)
    (Math|Integer|IncrementInt (Variables|/Game/Vehicles/BP_Kart.BP_Kart_C|GetlapsCompleted (Variables|Default|GetAs%20BP%20Kart_0))
      (:%20%20
        (Default|UpdateLaps (Variables|Default|GetAs%20BP%20Kart_0))
        (Default|EndRace _as_bp_kart_0_2)
        (Default|EndLap _as_bp_kart_0_2)
        (Utilities|FlowControl|Delay 2.0)
        (bind _returnvalue (UserInterface|CreateWidget "/Game/UI/WB_RaceComplete.WB_RaceComplete_C"))
        (UserInterface|Viewport|AddtoViewport _returnvalue 0)))
    (else
      (Default|StartLap _as_bp_kart_0_3)
      (Utilities|FlowControl|Delay 0.4)
      (Math|Integer|IncrementInt (Variables|/Game/Vehicles/BP_Kart.BP_Kart_C|GetlapsCompleted (Variables|Default|GetAs%20BP%20Kart_0))
        (:%20%20
          (Default|UpdateLaps (Variables|Default|GetAs%20BP%20Kart_0)))))))

(event EventBeginPlay
  (bind _asbp_kart (Utilities|Casting|CastToBP_Kart (Game|Player|GetPlayerPawn 0)))
  (Variables|Default|SetAs%20BP%20Kart_0 _asbp_kart))

(fn ConstructionScript)