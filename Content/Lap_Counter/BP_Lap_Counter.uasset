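; BP_Lap_Counter holds lap-counting logic for BP_Kart, but no event triggers it, so it never runs.
; The graph casts to BP_Kart and branches on IsFirstTime, whose true branch only sets the flag to true again.
; The false branch increments Laps and writes it to the kart's LapCounterUI text.
; A DoOnce, reset after a short delay, debounces repeat counts.
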(fn ConstructionScript)