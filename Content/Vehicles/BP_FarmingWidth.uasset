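; BP_FarmingWidth is an overlap-triggered actor in the vehicles folder that activates extra farming on a kart, likely as a farming-width pickup.
; When a BP_Kart begins overlapping it, it calls ActivateExtraFarming on that kart.
; It then sets its Active flag true and clears it after a three-second delay, without checking the flag itself.
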(event EventBeginPlay
  (|CallParentFunction) ; This node is disabled and will not be called.\nDrag off pins to build functionality.
)

(event Collision|EventActorBeginOverlap
  (params (OtherActor :type Actor%20Object%20Reference))
  (bind _asbp_kart (Utilities|Casting|CastToBP_Kart OtherActor))
  (Default|ActivateExtraFarming _asbp_kart)
  (Variables|Default|Setactive true)
  (Utilities|FlowControl|Delay 3.0)
  (Variables|Default|Setactive false))

(event EventTick
  (params (DeltaSeconds :type Float%20%28single-precision%29))
  (|CallParentFunction DeltaSeconds) ; This node is disabled and will not be called.\nDrag off pins to build functionality.
)

(fn ConstructionScript
  (|CallParentFunction))