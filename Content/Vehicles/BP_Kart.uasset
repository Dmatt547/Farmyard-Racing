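; Drivable physics kart for a lap-based farming race, with race and lap timers, lap counting and timed speed and extra-farming boosts.
; Each tick, per-wheel line traces push forces into a Box body for suspension, gravity and drive, while Enhanced Input feeds throttle and steering torque.
; It also spawns BP_planting beneath a Cone every tick and grows a farming percentage from throttle while a trace detects BP_Track.
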(event Custom|Start%20Race
  ;[1 1 1] Race Timer
  (bind _time (Timeline|Race%20time Play)
    (:Update
      (Variables|Default|SetRaceTime%20as%20Text (Utilities|TimeasText _time)))))

(event Custom|End%20Race
  ;[1 1 1] Race Timer
  (bind _time (Timeline|Race%20time Stop)
    (:Update
      (Variables|Default|SetRaceTime%20as%20Text (Utilities|TimeasText _time)))))

(event Custom|Start%20Lap
  (bind _time (Timeline|Lap%20time PlayFromStart)
    (:Update
      (bind _output_get (Variables|Default|SetLapTime _time))
      (Variables|Default|SetLapTimeAsText (Utilities|TimeasText _output_get)))))

(event Custom|End%20lap
  (bind _time (Timeline|Lap%20time Stop)
    (:Update
      (bind _output_get (Variables|Default|SetLapTime _time))
      (Variables|Default|SetLapTimeAsText (Utilities|TimeasText _output_get)))))

(event Custom|Update%20Laps
  (bind _lapscompleted (Variables|Default|GetlapsCompleted))
  (bind _lapsrequired (Variables|Default|GetLapsRequired))
  (Variables|Default|SetLaps%20Text (Utilities|LapsasText _lapscompleted _lapsrequired))
  (if (>= _lapscompleted _lapsrequired)
    (Variables|Default|SetRaceComplete? true)
    (else
      (Variables|Default|SetLapCompleted? true))))

(event Custom|Farm
  (bind _cone (Variables|Default|GetCone))
  (bind _returnvalue (Transformation|GetWorldLocation _cone))
  (bind _outhit (Collision|LineTraceByChannel (+ _returnvalue "0.000000,0.000000,100.000000") (- _returnvalue "0.000000,0.000000,100.000000") "TraceTypeQuery1" true 0 "None"))
  (Game|SpawnActorfromClass "/Game/Vehicles/BP_planting.BP_planting_C" (Math|Transform|MakeTransform (.Location (Collision|BreakHitResult _outhit)) (Transformation|GetActorRotation) (Math|Vector|MakeVector 1.0 (Variables|Default|GetFarming%20width) 0.1)) "Undefined" "MultiplyWithRoot" 0 0))

(event Custom|Activate%20Speed%20Boost
  (Variables|Default|SetAccelerationInput 1.0)
  (bind _returnvalue (Niagara|SpawnSystemAttached "/Game/sA_PickupSet_1/Fx/NiagaraSystems/NS_Energy_2.NS_Energy_2" (Variables|Default|GetBox) "spine_03" "0, 0, 0" "0, 0, 0" "KeepRelativeOffset" false))
  (Utilities|FlowControl|Delay 3.0)
  (Components|DestroyComponent _returnvalue))

(event Custom|Activate%20Extra%20Farming
  (Variables|Default|SetFarmingActive true)
  (Variables|Default|SetFarming%20width 1.0)
  (Utilities|FlowControl|Delay 3.0)
  (Variables|Default|SetFarming%20width 0.5)
  (Variables|Default|SetFarmingActive false))

(event Input|EnhancedActionEvents|EnhancedInputActionIA_Accelerate
  (params (ActionValue :type Float%20%28double-precision%29) (ElapsedSeconds :type Float%20%28double-precision%29) (TriggeredSeconds :type Float%20%28double-precision%29) (InputAction :type Input%20Action%20Object%20Reference :default "/Game/Inputs/IA_Accelerate.IA_Accelerate"))
  (Variables|Default|SetAccelerationInput (Math|Interpolation|FInterpTo (Variables|Default|GetAccelerationInput) ActionValue (Utilities|Time|GetWorldDeltaSeconds) 0.7)))

(event Input|EnhancedActionEvents|EnhancedInputActionIA_Steer
  (params (ActionValue :type Float%20%28double-precision%29) (ElapsedSeconds :type Float%20%28double-precision%29) (TriggeredSeconds :type Float%20%28double-precision%29) (InputAction :type Input%20Action%20Object%20Reference :default "/Game/Inputs/IA_Steer.IA_Steer"))
  (bind _acceleration (Variables|Default|GetAcceleration))
  (bind _box (Variables|Default|GetBox))
  (bind _accelerationinput (Variables|Default|GetAccelerationInput))
  (bind _returnvalue (Physics|GetMass _box))
  (bind _returnvalue_2 (- 2.0 _acceleration))
  (bind _returnvalue_3 (* ActionValue 4e+04 _returnvalue _accelerationinput _returnvalue_2))
  (bind _returnvalue_4 (/ _returnvalue_3 1e+04))
  (bind _returnvalue_5 (< _returnvalue_4 0.0))
  (Class|PrimitiveComponent|AddTorqueinRadians (Variables|Default|GetBox) (Math|Vector|MakeVector 0.0 0.0 _returnvalue_3) "None" false)
  (Transformation|SetRelativeRotation (Variables|Default|GetFL_Wheel) (Math|Rotator|MakeRotator 0.0 0.0 (Math|Interpolation|FInterpTo (.yaw (Variables|/Script/Engine.SceneComponent|GetRelativeRotation (Variables|Default|GetFR_Wheel))) (Math|Float|SelectFloat (Math|Float|SelectFloat -3e+01 3e+01 _returnvalue_5) (Math|Float|SelectFloat 3e+01 -3e+01 _returnvalue_5) (> _accelerationinput 0.0)) (Utilities|Time|GetWorldDeltaSeconds) 4.0)) false false))

(event Input|EnhancedActionEvents|EnhancedInputActionIA_Reset
  (params (ActionValue :type Boolean) (ElapsedSeconds :type Float%20%28double-precision%29) (TriggeredSeconds :type Float%20%28double-precision%29) (InputAction :type Input%20Action%20Object%20Reference :default "/Game/Inputs/IA_Reset.IA_Reset"))
  (bind _box (Variables|Default|GetBox))
  (bind _returnvalue (Transformation|GetWorldLocation _box))
  (Transformation|SetRelativeRotation _box (Math|Rotator|MakeRotator 0.0 0.0 (.yaw (Variables|/Script/Engine.SceneComponent|GetRelativeRotation _box))) false false)
  (Transformation|SetRelativeLocation (Variables|Default|GetBox) (Math|Vector|MakeVector (.x _returnvalue) (.y _returnvalue) (+ (.z _returnvalue) 2e+01)) false false))

(event EventBeginPlay
  (Input|AddMappingContext (PlayerController|LocalPlayerSubsystems|GetEnhancedInputLocalPlayerSubsystem (Game|GetPlayerController 0)) "/Game/Inputs/IMC_Vehicle.IMC_Vehicle" 0 "(bIgnoreAllPressedKeysUntilRelease=True,bForceImmediately=False,bNotifyUserSettings=False)")
  (bind _output_get (Variables|Default|SetLapsRequired (Variables|Default|GetLapsRequired)))
  (bind _output_get_2 (Variables|Default|SetlapsCompleted 0))
  (Variables|Default|SetLaps%20Text (Utilities|LapsasText _output_get_2 _output_get)))

(event EventTick
  (params (DeltaSeconds :type Float%20%28single-precision%29))
  (bind _returnvalue (Game|GetPlayerCameraManager 0))
  (CallFunction|SuspensionCast (Variables|Default|GetFL_Wheel))
  (CallFunction|SuspensionCast (Variables|Default|GetFR_Wheel))
  (CallFunction|SuspensionCast (Variables|Default|GetBR_Wheel))
  (CallFunction|SuspensionCast (Variables|Default|GetBL_Wheel))
  (CallFunction|CalculateAcceleration)
  (CallFunction|GravityCast (Variables|Default|GetFL_Wheel))
  (CallFunction|GravityCast (Variables|Default|GetFR_Wheel))
  (CallFunction|GravityCast (Variables|Default|GetBR_Wheel))
  (CallFunction|GravityCast (Variables|Default|GetBL_Wheel))
  (Variables|/Script/Engine.PlayerCameraManager|SetViewPitchMax _returnvalue 6e+01)
  (Variables|/Script/Engine.PlayerCameraManager|SetViewPitchMin _returnvalue -6e+01)
  (Variables|/Script/Engine.PlayerCameraManager|SetViewRollMax _returnvalue 6e+01)
  (Variables|/Script/Engine.PlayerCameraManager|SetViewRollMin _returnvalue 6e+01)
  (CallFunction|Farm)
  (CallFunction|TrackCollisionDetection)
  (CallFunction|CalculateFarmingPercentage))

(event Input|KeyboardEvents|D
  (params (Key :type Key%20Structure))
  (:Released
    (Transformation|SetRelativeRotation (Variables|Default|GetFR_Wheel) "0, 0, 0" false false)))

(event Input|KeyboardEvents|A
  (params (Key :type Key%20Structure))
  (:Released
    (Transformation|SetRelativeRotation (Variables|Default|GetFR_Wheel) "0, 0, 0" false false)))

(event Input|KeyboardEvents|Left
  (params (Key :type Key%20Structure))
  (:Released
    (Transformation|SetRelativeRotation (Variables|Default|GetFR_Wheel) "0, 0, 0" false false)))

(event Input|KeyboardEvents|Right
  (params (Key :type Key%20Structure))
  (:Released
    (Transformation|SetRelativeRotation (Variables|Default|GetFR_Wheel) "0, 0, 0" false false)))

(event Input|KeyboardEvents|1
  (params (Key :type Key%20Structure))
  (:Pressed
    (bind _returnvalue (UserInterface|CreateWidget "/Game/UI/WB_MainMenu.WB_MainMenu_C"))
    (UserInterface|Viewport|AddtoViewport _returnvalue 0)
    (Variables|/Script/Engine.PlayerController|SetbShowMouseCursor (Game|GetPlayerController 0) true)))

(fn ConstructionScript)

(fn SuspensionCast
  (params (WheelComp :type Scene%20Component%20Object%20Reference))
  (bind _returnvalue (Transformation|GetWorldLocation WheelComp))
  (bind _returnvalue_2 (Components|GetChildComponent WheelComp 0))
  (bind _outhit (Collision|LineTraceByChannel _returnvalue (+ _returnvalue (* (Math|Vector|GetUpVector WheelComp) -6e+01)) "TraceTypeQuery1" false 0 "None"))
  (if (.bBlockingHit (Collision|BreakHitResult _outhit))
    (Class|PrimitiveComponent|AddForceatLocation (Variables|Default|GetBox) (* (- 1.0 (Math|Float|NormalizetoRange (.Distance (Collision|BreakHitResult _outhit)) 0.0 6e+01)) (Math|Vector|GetUnitDirection(Vector) (.TraceEnd (Collision|BreakHitResult _outhit)) (.TraceStart (Collision|BreakHitResult _outhit))) 1e+05) (Transformation|GetWorldLocation WheelComp) "None")
    (CallFunction|AccelerateKart WheelComp)
    (Transformation|SetRelativeLocation _returnvalue_2 (Math|Vector|MakeVector 0.0 0.0 (Math|Interpolation|FInterpTo (.z (Variables|/Script/Engine.SceneComponent|GetRelativeLocation _returnvalue_2)) (+ (* (.Distance (Collision|BreakHitResult _outhit)) -1.0) 32.0) (Utilities|Time|GetWorldDeltaSeconds) 3.0)) false false)
    (else
      (CallFunction|AccelerateKart WheelComp))))

(fn CalculateAcceleration
  (Variables|Default|SetAcceleration (* (Math|Float|Lerp 0.0 0.0 (Variables|Default|GetAccelerationInput)) (Variables|Default|GetAccelerationInput)))
  (bind _output_get (Variables|Default|SetAccelerationInput (Math|Interpolation|FInterpTo (Variables|Default|GetAccelerationInput) 0.0 (Utilities|Time|GetWorldDeltaSeconds) 0.5)))
  (Transformation|AddLocalRotation (Variables|Default|GetWheel_BL) (Math|Rotator|MakeRotator 0.0 0.0 (Math|Interpolation|FInterpTo (Math|Float|SelectFloat -1e+03 1e+03 (> _output_get 0.0)) (Math|Float|SelectFloat -1e+03 1e+03 (> _output_get 0.0)) 0.0 0.0)) false false))

(fn AccelerateKart
  (params (WheelComp :type Scene%20Component%20Object%20Reference))
  (bind _box (Variables|Default|GetBox))
  (Class|PrimitiveComponent|AddForceatLocation (Variables|Default|GetBox) (* (Math|Vector|GetForwardVector _box) 1.5e+04 (Variables|Default|GetAccelerationInput) (Physics|GetMass _box)) (Transformation|GetWorldLocation WheelComp) "None")
  (Class|PrimitiveComponent|SetCenterOfMass (Variables|Default|GetBox) (* "-50.000000,0.000000,0.000000" (Variables|Default|GetAccelerationInput)) "None"))

(fn GravityCast
  (params (Wheel%20Comp :type Scene%20Component%20Object%20Reference))
  (bind _returnvalue (Transformation|GetWorldLocation Wheel%20Comp))
  (bind _outhit (Collision|LineTraceByChannel _returnvalue (+ _returnvalue (* (Math|Vector|GetUpVector Wheel%20Comp) -6e+02)) "TraceTypeQuery1" false 0 "None"))
  (if (.bBlockingHit (Collision|BreakHitResult _outhit))
    (Class|PrimitiveComponent|AddForceatLocation (Variables|Default|GetBox) (* (- 1.0 (Math|Float|NormalizetoRange (.Distance (Collision|BreakHitResult _outhit)) 0.0 6e+01)) (Math|Vector|GetUnitDirection(Vector) (.TraceStart (Collision|BreakHitResult _outhit)) (.TraceEnd (Collision|BreakHitResult _outhit))) -2e+04) (Transformation|GetWorldLocation Wheel%20Comp) "None")
    (else
      (CallFunction|AccelerateKart Wheel%20Comp))))

(fn TrackCollisionDetection
  (bind _cone (Variables|Default|GetCone))
  (bind _returnvalue (Transformation|GetWorldLocation _cone))
  (bind _outhit (Collision|LineTraceByChannel _returnvalue (+ _returnvalue "0.000000,0.000000,-100.000000") "TraceTypeQuery1" true 0 "None"))
  (Utilities|Casting|CastToBP_Track (.HitActor (Collision|BreakHitResult _outhit))
    (:then
      (Variables|Default|Seton%20track true)
      (Variables|Default|SetFarmingCompletion 0.5))
    (:CastFailed
      (Variables|Default|Seton%20track false))))

(fn CalculateFarmingPercentage
  (bind _accelerationinput (Variables|Default|GetAccelerationInput))
  (if (not (> (Variables|Default|GetlapsCompleted) (Variables|Default|GetLapsRequired)))
    (bind _output_get (Variables|Default|SetFarmingCompletionPercentage (Math|Float|SelectFloat (+ (Variables|Default|GetFarmingCompletionPercentage) (Math|Float|SelectFloat (/ (* _accelerationinput (Math|Float|SelectFloat 2.0 (Variables|Default|GetFarmingCompletion) (Variables|Default|GetFarmingActive))) 3e+01) 0.0 (> _accelerationinput 0.0))) (Variables|Default|GetFarmingCompletionPercentage) (Variables|Default|Geton%20track))))
    (Variables|Default|SetFarmingPrecentage (Utilities|Text|ToText(Float) _output_get "HalfToEven"))))