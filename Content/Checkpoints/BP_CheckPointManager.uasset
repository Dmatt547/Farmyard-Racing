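; Checkpoint manager for a kart race that counts checkpoint hits and resets the checkpoints after each completed lap.
; On BeginPlay it binds to every actor in its Checkpoints array and writes the hit/required progress to the player kart's CheckpointText.
; Once all are hit, a looping one-second timer, never cleared here, polls the kart's LapCompleted flag.
; When set, it clears the flag, unhides checkpoints, re-enables their collision and zeroes the count.
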(event Custom|CheckpointHit
  (bind _checkpointcount (Variables|Default|GetCheckpointCount))
  (bind _checkpoints_required (Variables|Default|GetCheckpoints%20Required))
  (Development|PrintString "Checkpoint Hit")
  (Math|Integer|IncrementInt _checkpointcount
    (:%20%20
      (Variables|/Game/Vehicles/BP_Kart.BP_Kart_C|Setcheckpoint%20Text (Variables|Default|GetAs%20BP%20Kart) (Utilities|CheckpointstoText _checkpoints_required _checkpointcount))
      (if (>= _checkpointcount _checkpoints_required)
        (Utilities|Time|SetTimerbyEvent (delegate Custom|ResetCheckpoints) 1.0 true)))))

(event Custom|ResetCheckpoints
  (bind _as_bp_kart (Variables|Default|GetAs%20BP%20Kart))
  (if (Variables|/Game/Vehicles/BP_Kart.BP_Kart_C|GetLapCompleted? _as_bp_kart)
    (Variables|/Game/Vehicles/BP_Kart.BP_Kart_C|SetLapCompleted? _as_bp_kart false)
    (for _array_element (Variables|Default|GetCheckpoints)
      (Rendering|SetActorHiddenInGame _array_element false)
      (Collision|SetCollisionEnabled (Variables|/Game/Checkpoints/BP_Checkpoint.BP_Checkpoint_C|GetCylinder _array_element) "QueryOnly")
      (bind _output_get (Variables|Default|SetCheckpointCount 0))
      (Variables|/Game/Vehicles/BP_Kart.BP_Kart_C|Setcheckpoint%20Text (Variables|Default|GetAs%20BP%20Kart) (Utilities|CheckpointstoText (Variables|Default|GetCheckpoints%20Required) _output_get)))))

(event EventBeginPlay
  (bind _checkpoints (Variables|Default|GetCheckpoints))
  (bind _asbp_kart (Utilities|Casting|CastToBP_Kart (Game|Player|GetPlayerPawn 0)))
  (Variables|Default|SetAs%20BP%20Kart _asbp_kart)
  (Variables|Default|SetCheckpoints%20Required (Utilities|Array|Length _checkpoints))
  (for _array_element _checkpoints
    (EventDispatchers|BindEventtoCheckpointHit _array_element (delegate Custom|CheckpointHit))
    (Variables|/Game/Vehicles/BP_Kart.BP_Kart_C|Setcheckpoint%20Text (Variables|Default|GetAs%20BP%20Kart) (Utilities|CheckpointstoText (Variables|Default|GetCheckpoints%20Required)))))

(fn ConstructionScript)